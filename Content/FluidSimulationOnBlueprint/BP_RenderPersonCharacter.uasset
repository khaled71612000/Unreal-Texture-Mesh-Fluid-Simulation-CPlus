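; First-person character that paints into the RT_Density render target for a fluid simulation, clearing it on BeginPlay.
; While E is held, Tick line-traces from the actor along the camera's forward vector.
; Hits on TargetCameraActor become collision UVs, where M_SnowFlake is drawn as a brush, relying on complex tracing and project-enabled UV hit support.
; Q toggles turbulence, which draws M_Tirbulence over the whole target every frame.
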(event EventBeginPlay
  (Rendering|ClearRenderTarget2D "/Game/FluidSimulationOnBlueprint/RT_Density.RT_Density"))

(event EventTick
  (params (DeltaSeconds :type Float%20%28single-precision%29))
  ;[1 1 1] Render first stage
  (if (Variables|Default|GetisPainting)
    (CallFunction|ShootPaint))
  ;[1 1 1] tirbulence second staghe
  (if (Variables|Default|GetIsTurblent)
    (CallFunction|AddTurbulence)))

(event Input|KeyboardEvents|E
  (params (Key :type Key%20Structure :default "None"))
  (:Pressed
    (Variables|Default|SetisPainting true))
  (:Released
    (Variables|Default|SetisPainting false)))

(event Input|KeyboardEvents|Q
  (params (Key :type Key%20Structure :default "None"))
  (:Released
    (Variables|Default|SetIsTurblent (not (Variables|Default|GetIsTurblent)))))

(fn ConstructionScript
  (|CallParentFunction))

(fn ShootPaint
  (bind _returnvalue (Transformation|GetActorLocation))
  (bind _brushsize (Variables|Default|GetBrushSize))
  ;[1 1 1] must be complex and enable uv hit on collision in project setttings
  (bind _outhit (Collision|LineTraceByChannel _returnvalue (+ _returnvalue (* (Math|Vector|GetForwardVector (Variables|Default|GetFirstPersonCamera)) (Variables|Default|GetTraceDistance))) "TraceTypeQuery1" true 0 "ForDuration" true "(R=1.000000,G=0.000000,B=0.000000,A=1.000000)" "(R=0.000000,G=1.000000,B=0.000000,A=1.000000)" 1.0))
  (if (== (.HitActor (Collision|BreakHitResult _outhit)) (Variables|Default|GetTargetCameraActor))
    ;[1 1 1] Get render target size on UV by multiplying
    (bind (_canvas _size _context) (Rendering|BeginDrawCanvastoRenderTarget "/Game/FluidSimulationOnBlueprint/RT_Density.RT_Density"))
    (Canvas|DrawMaterial :self _canvas :RenderMaterial "/Game/FluidSimulationOnBlueprint/M_SnowFlake.M_SnowFlake" :ScreenPosition (- (* _size (.UV (Class|GameplayStatics|FindCollisionUV _outhit))) (/ _brushsize "(X=2.000000,Y=2.000000)")) :ScreenSize _brushsize :CoordinateSize "(X=1.000000,Y=1.000000)" :PivotPoint "(X=0.500000,Y=0.500000)")
    (Rendering|EndDrawCanvastoRenderTarget _context)))

(fn AddTurbulence
  (bind (_canvas _size _context) (Rendering|BeginDrawCanvastoRenderTarget "/Game/FluidSimulationOnBlueprint/RT_Density.RT_Density"))
  (Canvas|DrawMaterial :self _canvas :RenderMaterial "/Game/FluidSimulationOnBlueprint/M_Tirbulence.M_Tirbulence" :ScreenSize _size :CoordinateSize "(X=1.000000,Y=1.000000)" :PivotPoint "(X=0.500000,Y=0.500000)")
  (Rendering|EndDrawCanvastoRenderTarget _context))